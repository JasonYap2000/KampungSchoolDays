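; BP_Menu3D is a 3D in-world menu actor that moves the player's view between linked menus.
; On BeginPlay it binds to its Menu3D_Widget's TransitionToLinkedMenu dispatcher, which passes an index into the LinkedMenus array.
; For a valid index it disables its own collision, enables the target menu's, and smoothly blends player 0's view target to that actor with a cubic blend.
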(event Custom|TransitionTo
  (params (3D%20Menu :type BP%20Menu%203D%20Object%20Reference))
  (Collision|SetActorEnableCollision false)
  (Collision|SetActorEnableCollision 3D%20Menu true)
  (Game|Player|SetViewTargetwithBlend (Game|GetPlayerController 0) 3D%20Menu 2.0 "VTBlend_Cubic" 2.0 false))

(event Custom|TransitionToLinkedMenu_Event_0
  (params (MenuIndex :type Integer))
  (if (Utilities|Array|IsValidIndex (Variables|Default|GetLinkedMenus) MenuIndex)
    (CallFunction|Transitionto (Utilities|Array|Get(acopy) (Variables|Default|GetLinkedMenus) MenuIndex))))

(event EventBeginPlay
  (bind _asmenu_3d_widget (Utilities|Casting|CastToMenu3D_Widget (UserInterface|GetUserWidgetObject (Variables|Default|GetWidget))))
  (EventDispatchers|AssignTransitiontoLinkedMenu _asmenu_3d_widget (delegate Custom|TransitionToLinkedMenu_Event_0)))

(fn ConstructionScript)