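; Player actor for the Guli marble minigame, running the whole turn-based match against an NPC, plus tutorial, pause and result screens.
; Player aims with A/D and mouse, then holds and releases click to launch with oscillating timeline power.
; NPC aims near the closest sphere-traced ball and fires at random power.
; Score boxes credit the current side for each Ball2; Tick ends the match once the round counter hits its limit.
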(event OnComponentBeginOverlap(ScoreBox1)
  (params (OverlappedComponent :type Primitive%20Component%20Object%20Reference) (OtherActor :type Actor%20Object%20Reference) (OtherComp :type Primitive%20Component%20Object%20Reference) (OtherBodyIndex :type Integer) (bFromSweep :type Boolean) (SweepResult :type Hit%20Result%20Structure%20%28by%20ref%29))
  ;[1 1 1] Overlap Get Score
  (bind _asball_2 (Utilities|Casting|CastToBall2 OtherActor))
  (if (Variables|Default|GetPlayer%20Turn%20?)
    (Variables|Default|SetPlayer%20Score (+ (Variables|Default|GetPlayer%20Score) 1))
    (Development|PrintString "Player score + 1")
    (Utilities|FlowControl|Delay 0.0)
    (Actor|DestroyActor _asball_2)
    (else
      (Variables|Default|SetNPC%20Score (+ (Variables|Default|GetNPC%20Score) 1))
      (Development|PrintString "NPC score + 1")
      (Utilities|FlowControl|Delay 0.0)
      (Actor|DestroyActor _asball_2)))
  (Audio|PlaySound2D "/Game/Audio/SE/collect.collect" 1.0 1.0 0.0 0 0))

(event OnComponentHit(Sphere)
  (params (HitComponent :type Primitive%20Component%20Object%20Reference) (OtherActor :type Actor%20Object%20Reference) (OtherComp :type Primitive%20Component%20Object%20Reference) (NormalImpulse :type Vector :default "0, 0, 0") (Hit :type Hit%20Result%20Structure%20%28by%20ref%29)))

(event OnComponentBeginOverlap(Sphere1)
  (params (OverlappedComponent :type Primitive%20Component%20Object%20Reference) (OtherActor :type Actor%20Object%20Reference) (OtherComp :type Primitive%20Component%20Object%20Reference) (OtherBodyIndex :type Integer) (bFromSweep :type Boolean) (SweepResult :type Hit%20Result%20Structure%20%28by%20ref%29))
  (Utilities|Casting|CastToBall2 OtherActor)
  (Audio|PlaySoundatLocation "/Game/Minigame/Guli/Guli_hitsound_Cue.Guli_hitsound_Cue" (Transformation|GetWorldLocation (Variables|Default|GetSphere)) "0, 0, 0" 1.0 1.0 0.0 0 0 0)
  ;[1 1 1] Play Sound Here
  (Development|PrintString "HIT" true true "(R=0.000000,G=0.660000,B=1.000000,A=1.000000)" 5.0))

(event OnComponentBeginOverlap(ScoreBox2)
  (params (OverlappedComponent :type Primitive%20Component%20Object%20Reference) (OtherActor :type Actor%20Object%20Reference) (OtherComp :type Primitive%20Component%20Object%20Reference) (OtherBodyIndex :type Integer) (bFromSweep :type Boolean) (SweepResult :type Hit%20Result%20Structure%20%28by%20ref%29))
  ;[1 1 1] Overlap Get Score
  (bind _asball_2 (Utilities|Casting|CastToBall2 OtherActor))
  (if (Variables|Default|GetPlayer%20Turn%20?)
    (Variables|Default|SetPlayer%20Score (+ (Variables|Default|GetPlayer%20Score) 1))
    (Development|PrintString "Player score + 1")
    (Utilities|FlowControl|Delay 0.0)
    (Actor|DestroyActor _asball_2)
    (else
      (Variables|Default|SetNPC%20Score (+ (Variables|Default|GetNPC%20Score) 1))
      (Development|PrintString "NPC score + 1")
      (Utilities|FlowControl|Delay 0.0)
      (Actor|DestroyActor _asball_2)))
  (Audio|PlaySound2D "/Game/Audio/SE/collect.collect" 1.0 1.0 0.0 0 0))

(event OnComponentBeginOverlap(ScoreBox3)
  (params (OverlappedComponent :type Primitive%20Component%20Object%20Reference) (OtherActor :type Actor%20Object%20Reference) (OtherComp :type Primitive%20Component%20Object%20Reference) (OtherBodyIndex :type Integer) (bFromSweep :type Boolean) (SweepResult :type Hit%20Result%20Structure%20%28by%20ref%29))
  ;[1 1 1] Overlap Get Score
  (bind _asball_2 (Utilities|Casting|CastToBall2 OtherActor))
  (if (Variables|Default|GetPlayer%20Turn%20?)
    (Variables|Default|SetPlayer%20Score (+ (Variables|Default|GetPlayer%20Score) 1))
    (Development|PrintString "Player score + 1")
    (Utilities|FlowControl|Delay 0.0)
    (Actor|DestroyActor _asball_2)
    (else
      (Variables|Default|SetNPC%20Score (+ (Variables|Default|GetNPC%20Score) 1))
      (Development|PrintString "NPC score + 1")
      (Utilities|FlowControl|Delay 0.0)
      (Actor|DestroyActor _asball_2)))
  (Audio|PlaySound2D "/Game/Audio/SE/collect.collect" 1.0 1.0 0.0 0 0))

(event OnComponentBeginOverlap(ScoreBox4)
  (params (OverlappedComponent :type Primitive%20Component%20Object%20Reference) (OtherActor :type Actor%20Object%20Reference) (OtherComp :type Primitive%20Component%20Object%20Reference) (OtherBodyIndex :type Integer) (bFromSweep :type Boolean) (SweepResult :type Hit%20Result%20Structure%20%28by%20ref%29))
  ;[1 1 1] Overlap Get Score
  (bind _asball_2 (Utilities|Casting|CastToBall2 OtherActor))
  (if (Variables|Default|GetPlayer%20Turn%20?)
    (Variables|Default|SetPlayer%20Score (+ (Variables|Default|GetPlayer%20Score) 1))
    (Development|PrintString "Player score + 1")
    (Utilities|FlowControl|Delay 0.0)
    (Actor|DestroyActor _asball_2)
    (else
      (Variables|Default|SetNPC%20Score (+ (Variables|Default|GetNPC%20Score) 1))
      (Development|PrintString "NPC score + 1")
      (Utilities|FlowControl|Delay 0.0)
      (Actor|DestroyActor _asball_2)))
  (Audio|PlaySound2D "/Game/Audio/SE/collect.collect" 1.0 1.0 0.0 0 0))

(event OnComponentBeginOverlap(ScoreBox5)
  (params (OverlappedComponent :type Primitive%20Component%20Object%20Reference) (OtherActor :type Actor%20Object%20Reference) (OtherComp :type Primitive%20Component%20Object%20Reference) (OtherBodyIndex :type Integer) (bFromSweep :type Boolean) (SweepResult :type Hit%20Result%20Structure%20%28by%20ref%29))
  ;[1 1 1] Overlap Get Score
  (bind _asball_2 (Utilities|Casting|CastToBall2 OtherActor))
  (if (Variables|Default|GetPlayer%20Turn%20?)
    (Variables|Default|SetPlayer%20Score (+ (Variables|Default|GetPlayer%20Score) 1))
    (Development|PrintString "Player score + 1")
    (Utilities|FlowControl|Delay 0.0)
    (Actor|DestroyActor _asball_2)
    (else
      (Variables|Default|SetNPC%20Score (+ (Variables|Default|GetNPC%20Score) 1))
      (Development|PrintString "NPC score + 1")
      (Utilities|FlowControl|Delay 0.0)
      (Actor|DestroyActor _asball_2)))
  (Audio|PlaySound2D "/Game/Audio/SE/collect.collect" 1.0 1.0 0.0 0 0))

(event OnComponentBeginOverlap(ScoreBox6)
  (params (OverlappedComponent :type Primitive%20Component%20Object%20Reference) (OtherActor :type Actor%20Object%20Reference) (OtherComp :type Primitive%20Component%20Object%20Reference) (OtherBodyIndex :type Integer) (bFromSweep :type Boolean) (SweepResult :type Hit%20Result%20Structure%20%28by%20ref%29))
  ;[1 1 1] Overlap Get Score
  (bind _asball_2 (Utilities|Casting|CastToBall2 OtherActor))
  (if (Variables|Default|GetPlayer%20Turn%20?)
    (Variables|Default|SetPlayer%20Score (+ (Variables|Default|GetPlayer%20Score) 1))
    (Development|PrintString "Player score + 1")
    (Utilities|FlowControl|Delay 0.0)
    (Actor|DestroyActor _asball_2)
    (else
      (Variables|Default|SetNPC%20Score (+ (Variables|Default|GetNPC%20Score) 1))
      (Development|PrintString "NPC score + 1")
      (Utilities|FlowControl|Delay 0.0)
      (Actor|DestroyActor _asball_2)))
  (Audio|PlaySound2D "/Game/Audio/SE/collect.collect" 1.0 1.0 0.0 0 0))

(event OnComponentBeginOverlap(ScoreBox7)
  (params (OverlappedComponent :type Primitive%20Component%20Object%20Reference) (OtherActor :type Actor%20Object%20Reference) (OtherComp :type Primitive%20Component%20Object%20Reference) (OtherBodyIndex :type Integer) (bFromSweep :type Boolean) (SweepResult :type Hit%20Result%20Structure%20%28by%20ref%29))
  ;[1 1 1] Overlap Get Score
  (bind _asball_2 (Utilities|Casting|CastToBall2 OtherActor))
  (if (Variables|Default|GetPlayer%20Turn%20?)
    (Variables|Default|SetPlayer%20Score (+ (Variables|Default|GetPlayer%20Score) 1))
    (Development|PrintString "Player score + 1")
    (Utilities|FlowControl|Delay 0.0)
    (Actor|DestroyActor _asball_2)
    (else
      (Variables|Default|SetNPC%20Score (+ (Variables|Default|GetNPC%20Score) 1))
      (Development|PrintString "NPC score + 1")
      (Utilities|FlowControl|Delay 0.0)
      (Actor|DestroyActor _asball_2)))
  (Audio|PlaySound2D "/Game/Audio/SE/collect.collect" 1.0 1.0 0.0 0 0))

(event OnComponentBeginOverlap(ScoreBox8)
  (params (OverlappedComponent :type Primitive%20Component%20Object%20Reference) (OtherActor :type Actor%20Object%20Reference) (OtherComp :type Primitive%20Component%20Object%20Reference) (OtherBodyIndex :type Integer) (bFromSweep :type Boolean) (SweepResult :type Hit%20Result%20Structure%20%28by%20ref%29))
  ;[1 1 1] Overlap Get Score
  (bind _asball_2 (Utilities|Casting|CastToBall2 OtherActor))
  (if (Variables|Default|GetPlayer%20Turn%20?)
    (Variables|Default|SetPlayer%20Score (+ (Variables|Default|GetPlayer%20Score) 1))
    (Development|PrintString "Player score + 1")
    (Utilities|FlowControl|Delay 0.0)
    (Actor|DestroyActor _asball_2)
    (else
      (Variables|Default|SetNPC%20Score (+ (Variables|Default|GetNPC%20Score) 1))
      (Development|PrintString "NPC score + 1")
      (Utilities|FlowControl|Delay 0.0)
      (Actor|DestroyActor _asball_2)))
  (Audio|PlaySound2D "/Game/Audio/SE/collect.collect" 1.0 1.0 0.0 0 0))

(event Custom|TestEnum
  (switch Utilities|FlowControl|Switch|SwitchonTurn_Enum (Variables|Default|GetCurrentTurn)
    (:NewEnumerator0
      (Development|PrintString "Player Turn")
      (bind _returnvalue (UserInterface|CreateWidget "/Game/Minigame/Guli/PlayerTurn_UI.PlayerTurn_UI_C"))
      (UserInterface|Viewport|AddtoViewport _returnvalue 0)
      (Variables|Default|SetPlayer%20Turn%20? true)
      (Variables|Default|SetNPC%20Turn%20? false)
      (Components|Arrow|SetArrowColor(LinearColor) (Variables|Default|GetArrow) "(R=0.000000,G=0.000000,B=1.000000,A=1.000000)")
      (Transformation|SetWorldTransform (Variables|Default|GetBox) (Transformation|GetWorldTransform (Variables|Default|GetPlayer%20Point)) false false)
      (Utilities|FlowControl|DoOnce false) ; enters at Reset
    )
    (:NewEnumerator1
      (Development|PrintString "NPC Turn")
      (bind _returnvalue_2 (UserInterface|CreateWidget "/Game/Minigame/Guli/NPCTurn_UI1.NPCTurn_UI1_C"))
      (UserInterface|Viewport|AddtoViewport _returnvalue_2 0)
      (Variables|Default|SetPlayer%20Turn%20? false)
      (Components|Arrow|SetArrowColor(LinearColor) (Variables|Default|GetArrow) "(R=1.000000,G=0.000000,B=0.000000,A=1.000000)")
      (Transformation|SetWorldTransform (Variables|Default|GetBox) (Transformation|GetWorldTransform (Variables|Default|GetNPC%20Point)) false false)
      (Utilities|FlowControl|Delay 1.5)
      (Variables|Default|SetNPC%20Turn%20? true))))

(event Custom|CallTutorial2
  (Audio|PlaySound2D "/Game/Audio/SE/OpenBook_CUe.OpenBook_CUe" 1.0 1.0 0.0 0 0)
  (UserInterface|Viewport|AddtoViewport (Variables|Default|GetGuli_TutorialWidget2) 0))

(event Custom|CallTutorial1
  (Audio|PlaySound2D "/Game/Audio/SE/CloseBook_CUe.CloseBook_CUe" 1.0 1.0 0.0 0 0)
  (UserInterface|Viewport|AddtoViewport (Variables|Default|GetGuli_TutorialWidget) 0))

(event EventTick
  (params (DeltaSeconds :type Float%20%28single-precision%29))
  (bind _sphere (Variables|Default|GetSphere))
  (bind _sphere_2 (Variables|Default|GetSphere))
  (bind _sphere_3 (Variables|Default|GetSphere))
  (bind _arrow (Variables|Default|GetArrow))
  (bind _arrow_2 (Variables|Default|GetArrow))
  (bind _returnvalue (Transformation|GetWorldLocation _arrow_2))
  (if (>= (Variables|Default|GetPlayingTurn) 6)
    ;[1 1 1] GameEnd_Result
    (if (> (Variables|Default|GetPlayer%20Score) (Variables|Default|GetNPC%20Score))
      (Input|DisableInput (Game|GetPlayerController 0))
      (Game|SetGamePaused true)
      (Variables|/Script/Engine.PlayerController|SetbShowMouseCursor (Game|GetPlayerController 0) true)
      (bind _returnvalue_2 (UserInterface|CreateWidget "/Game/Minigame/Guli/Goli_WinUI.Goli_WinUI_C"))
      (UserInterface|Viewport|AddtoViewport _returnvalue_2 0)
      (Audio|PlaySound2D "/Game/Audio/SE/Winning_Cue.Winning_Cue" 1.0 1.0 0.0 0 0)
      (elif (> (Variables|Default|GetNPC%20Score) (Variables|Default|GetPlayer%20Score))
        (Input|DisableInput (Game|GetPlayerController 0))
        (Game|SetGamePaused true)
        (Variables|/Script/Engine.PlayerController|SetbShowMouseCursor (Game|GetPlayerController 0) true)
        (bind _returnvalue_3 (UserInterface|CreateWidget "/Game/Minigame/Guli/Goli_LoseUI.Goli_LoseUI_C"))
        (UserInterface|Viewport|AddtoViewport _returnvalue_3 0)
        (Audio|PlaySound2D "/Game/Audio/SE/Lose_Cue.Lose_Cue" 1.0 1.0 0.0 0 0)
        (elif (== (Variables|Default|GetNPC%20Score) (Variables|Default|GetPlayer%20Score))
          (Input|DisableInput (Game|GetPlayerController 0))
          (Game|SetGamePaused true)
          (Variables|/Script/Engine.PlayerController|SetbShowMouseCursor (Game|GetPlayerController 0) true)
          (bind _returnvalue_4 (UserInterface|CreateWidget "/Game/Minigame/Guli/Goli_DrawUI.Goli_DrawUI_C"))
          (UserInterface|Viewport|AddtoViewport _returnvalue_4 0)
          (Audio|PlaySound2D "/Game/Audio/SE/Lose_Cue.Lose_Cue" 1.0 1.0 0.0 0 0))))
    (elif (Variables|Default|GetIsTutorial1?)
      (Utilities|FlowControl|DoOnce false
        (:Completed
          (Input|SetInputModeUIOnly (Game|GetPlayerController 0) 0 "DoNotLock")
          (UserInterface|Viewport|AddtoViewport (Variables|Default|GetGuli_TutorialWidget) 0)
          (Variables|/Script/Engine.PlayerController|SetbShowMouseCursor (Game|GetPlayerController 0) true)))
      (else
        (Input|SetInputModeGameOnly (Game|GetPlayerController 0))
        ;[1 1 1] player movement
        (Utilities|FlowControl|Sequence
          (:then_0
            (if (Variables|Default|GetTurnRight?)
              (Transformation|AddLocalRotation (Variables|Default|GetDefaultSceneRoot) "0.000000,-0.500000,0.000000" false false)))
          (:then_1
            (if (Variables|Default|GetTurnLeft?)
              (Transformation|AddLocalRotation (Variables|Default|GetDefaultSceneRoot) "0.000000,0.500000,0.000000" false false)))
          (:then_2
            (if (Variables|Default|GetNPC%20Turn%20?)
              (Utilities|FlowControl|Sequence
                (:then_0
                  (Utilities|FlowControl|DoOnce false :!label _label
                    (:Completed
                      (if (Math|Random|RandomBool)
                        (Variables|Default|SetTurnLeft? true)
                        (else
                          (Variables|Default|SetTurnRight? true)))
                      (Development|PrintString "NPC Move")
                      (bind _output_get (Variables|Default|Setrandom%20Float (Math|Random|RandomFloatinRange 1e+01 8e+01)))
                      (Development|PrintString (Utilities|String|ToString(Float) _output_get))
                      (Utilities|FlowControl|Delay (Math|Random|RandomFloatinRange 1.5 2.5))
                      (Variables|Default|SetTurnRight? false)
                      (Variables|Default|SetTurnLeft? false)
                      (Development|PrintString "npc stop")
                      (Utilities|FlowControl|Delay 1.5)
                      (Transformation|SetWorldTransform (Variables|Default|Geter) (Transformation|GetWorldTransform (Variables|Default|GetArrow2)) false false)
                      (Utilities|FlowControl|Delay 0.5)
                      (Transformation|SetWorldLocation _sphere_2 (Transformation|GetWorldLocation (Variables|Default|Getrespawn)) false true)
                      (Development|SetHiddeninGame _sphere_2 false false)
                      (Collision|SetCollisionEnabled _sphere_2 "QueryAndPhysics")
                      (Physics|SetSimulatePhysics _sphere true)
                      (Utilities|FlowControl|Sequence
                        (:then_0
                          (Development|PrintString "launch")
                          (Physics|AddImpulse _sphere (* (Math|Vector|GetForwardVector (Variables|Default|GetArrow)) (Math|Random|RandomFloatinRange 2e+03 2.5e+03)) "None" true)
                          (Utilities|FlowControl|Delay 1.0)
                          (bind _output_get_2 (Variables|Default|SetCanReset true))
                          (Utilities|FlowControl|Delay 6.0)
                          (if _output_get_2
                            (Variables|Default|SetCanReset false)
                            (Physics|SetSimulatePhysics _sphere_3 false)
                            (Development|SetHiddeninGame _sphere_3 true false)
                            (Collision|SetCollisionEnabled (Variables|Default|GetSphere) "NoCollision")
                            (Variables|Default|SetCanChangeDirection true)
                            (Transformation|SetWorldTransform (Variables|Default|Geter) (Transformation|GetWorldTransform (Variables|Default|GetArrow1)) false false)
                            (CallFunction|SwitchTurn)
                            (CallFunction|TestEnum)
                            (Utilities|FlowControl|Sequence
                              (:then_0
                                (goto _label Reset))
                              (:then_1
                                (goto _label_2 Reset)))))
                        (:then_1
                          (Audio|PlaySound2D "/Game/Audio/SE/Miss_cue.Miss_cue" 1.0 1.0 0.0 0 0))))))
                (:then_1
                  (bind _outhits (Collision|MultiSphereTraceForObjects _returnvalue _returnvalue (Math|Conversions|ToFloat(Integer) (Variables|Default|GetBallRadius)) (Utilities|Array|MakeArray "ObjectTypeQuery3") false (Utilities|Array|MakeArray self (Game|Player|GetPlayerPawn 0)) "None" true "(R=0.119134,G=0.000000,B=1.000000,A=1.000000)"))
                  (Variables|Default|SetClosestBall (.hitactor (Utilities|Array|Get(acopy) _outhits)))
                  (for _array_element _outhits
                    (if (< (Transformation|GetDistanceTo (.HitActor (Collision|BreakHitResult _array_element)) self) (Transformation|GetDistanceTo (Variables|Default|GetClosestBall) self))
                      (Variables|Default|SetClosestBall (.HitActor (Collision|BreakHitResult _array_element))))))
                (:then_2
                  (Transformation|SetWorldRotation _arrow (Math|Rotator|MakeRotator 0.0 0.0 (.yaw (Math|Rotator|FindLookatRotation (Transformation|GetWorldLocation _arrow) (+ (Transformation|GetActorLocation (Variables|Default|GetClosestBall)) (Variables|Default|Getrandom%20Float))))) false false)))))
          (:then_3
            (Utilities|FlowControl|DoOnce false :!label _label_2
              (:Completed
                (Variables|Default|SetPlayingTurn (+ (Variables|Default|GetPlayingTurn) 1)))))
          (:then_4
            (Utilities|FlowControl|DoOnce false
              (:Completed
                (bind _returnvalue_5 (UserInterface|CreateWidget "/Game/Minigame/Guli/PlayerTurn_UI.PlayerTurn_UI_C"))
                (UserInterface|Viewport|AddtoViewport _returnvalue_5 0)
                (bind _returnvalue_6 (UserInterface|CreateWidget "/Game/Minigame/Guli/Goli_ScoreUI.Goli_ScoreUI_C"))
                (UserInterface|Viewport|AddtoViewport _returnvalue_6 0)))))))))

(event EventBeginPlay
  (bind _self self)
  (Utilities|FlowControl|Sequence
    (:then_0
      (Variables|Default|SetCurrentTurn "NewEnumerator0")
      (bind _returnvalue (UserInterface|CreateWidget "/Game/World/WorldFadeIn.WorldFadeIn_C"))
      (UserInterface|Viewport|AddtoViewport _returnvalue 0))
    (:then_1
      (bind _returnvalue_2 (UserInterface|CreateWidget "/Game/Minigame/Guli/MiniGame1_TutorialWidget.MiniGame1_TutorialWidget_C"))
      (bind _output_get (Variables|Default|SetGuli_TutorialWidget _returnvalue_2))
      (Variables|/Game/Minigame/Guli/MiniGame1_TutorialWidget.MiniGame1_TutorialWidget_C|SetBP_player _output_get _self)
      (bind _returnvalue_3 (UserInterface|CreateWidget "/Game/Minigame/Guli/MiniGame1_TutorialWidget2.MiniGame1_TutorialWidget2_C"))
      (bind _output_get_2 (Variables|Default|SetGuli_TutorialWidget2 _returnvalue_3))
      (Variables|/Game/Minigame/Guli/MiniGame1_TutorialWidget2.MiniGame1_TutorialWidget2_C|SetBP_player _output_get_2 _self)
      (bind _returnvalue_4 (UserInterface|CreateWidget "/Game/Minigame/Guli/MiniGame1_SE_Widget.MiniGame1_SE_Widget_C"))
      (Variables|Default|SetMiniGame1SEWidget _returnvalue_4))
    (:then_2
      (bind _asplayer_game_instance (Utilities|Casting|CastToPlayer_GameInstance (Game|GetGameInstance)))
      (Variables|Default|SetIsTutorial1? (Variables|/Game/World/Player_GameInstance.Player_GameInstance_C|GetIsTutorial1? _asplayer_game_instance)))))

(event Input|MouseEvents|MouseX
  (params (AxisValue :type Float%20%28single-precision%29))
  (if (Variables|Default|GetPlayer%20Turn%20?)
    (Transformation|AddLocalRotation (Variables|Default|GetArrow) (Math|Rotator|MakeRotator 0.0 0.0 AxisValue) false false)))

(event Input|MouseEvents|RightMouseButton
  (params (Key :type Key%20Structure :default "None"))
  ;[1 1 1] no used
)

(event Input|KeyboardEvents|P
  (params (Key :type Key%20Structure :default "None")))

(event Input|KeyboardEvents|Escape
  (params (Key :type Key%20Structure :default "None"))
  (bind _minigame1sewidget (Variables|Default|GetMiniGame1SEWidget))
  (:Pressed
    (if (not (Variables|Default|GetIsLaunch?))
      (if (Variables|Default|GetIsPause?)
        (Variables|Default|SetIsPause? false)
        (Game|SetGamePaused false)
        (Variables|/Script/Engine.PlayerController|SetbShowMouseCursor (Game|GetPlayerController 0) false)
        (Widget|RemovefromParent _minigame1sewidget)
        (else
          (Variables|Default|SetIsPause? true)
          (Game|SetGamePaused true)
          (Development|PrintString "pause")
          (Variables|/Script/Engine.PlayerController|SetbShowMouseCursor (Game|GetPlayerController 0) true)
          (UserInterface|Viewport|AddtoViewport _minigame1sewidget 0))))))

(event Input|MouseEvents|LeftMouseButton
  (params (Key :type Key%20Structure :default "None"))
  (bind _sphere (Variables|Default|GetSphere))
  (bind _sphere_2 (Variables|Default|GetSphere))
  (bind _sphere_3 (Variables|Default|GetSphere))
  (:Pressed
    (Utilities|FlowControl|DoOnce false
      (:Completed
        (if (Variables|Default|GetPlayer%20Turn%20?)
          (Variables|Default|SetTurnLeft? false)
          (Variables|Default|SetIsLaunch? true)
          (Variables|Default|SetTurnRight? false)
          (Transformation|SetWorldTransform (Variables|Default|Geter) (Transformation|GetWorldTransform (Variables|Default|GetArrow2)) false false)
          (Variables|Default|SetCanChangeDirection false)
          (Utilities|FlowControl|Sequence
            (:then_0
              (bind _returnvalue (Audio|SpawnSound2D "/Game/Minigame/Guli/Charging_Cue.Charging_Cue" 1.0 1.0 0.0 0))
              (Variables|Default|SetAudioCom _returnvalue))
            (:then_1
              (bind _throwspeed (Timeline|Timeline_0 PlayFromStart)
                (:Update
                  (Variables|Default|SetThrow%20Speed _throwspeed))
                (:Finished
                  (bind _throwspeed_2 (Timeline|Timeline_1 ReverseFromEnd)
                    (:Update
                      (Variables|Default|SetThrow%20Speed _throwspeed_2))
                    (:Finished
                      (Timeline|Timeline_0 PlayFromStart)))))))))))
  (:Released
    (if (Variables|Default|GetPlayer%20Turn%20?)
      (Utilities|FlowControl|DoOnce false :!label _label
        (:Completed
          (Variables|Default|SetIsLaunch? false)
          (Audio|Components|Audio|Stop (Variables|Default|GetAudioCom))
          (Transformation|SetWorldLocation _sphere_3 (Transformation|GetWorldLocation (Variables|Default|Getrespawn)) false true)
          (Development|SetHiddeninGame _sphere_3 false false)
          (Collision|SetCollisionEnabled _sphere_3 "QueryAndPhysics")
          (Physics|SetSimulatePhysics _sphere_2 true)
          (Utilities|FlowControl|Sequence
            (:then_0
              (Development|PrintString "launch")
              (Physics|AddImpulse _sphere_2 (* (Math|Vector|GetForwardVector (Variables|Default|GetArrow)) (Variables|Default|GetThrow%20Speed)) "None" true)
              (Utilities|FlowControl|Delay 1.0)
              (Development|PrintString "can reset")
              (bind _output_get (Variables|Default|SetCanReset true))
              (Utilities|FlowControl|Delay 6.0)
              (if _output_get
                (Variables|Default|SetCanReset false)
                (Physics|SetSimulatePhysics _sphere false)
                (Development|SetHiddeninGame _sphere true false)
                (Collision|SetCollisionEnabled (Variables|Default|GetSphere) "NoCollision")
                (Variables|Default|SetCanChangeDirection true)
                (Transformation|SetWorldTransform (Variables|Default|Geter) (Transformation|GetWorldTransform (Variables|Default|GetArrow1)) false false)
                (Development|PrintString "change camera")
                (CallFunction|SwitchTurn)
                (CallFunction|TestEnum)
                (Utilities|FlowControl|Sequence
                  (:then_0
                    (goto _label Reset))
                  (:then_1
                    (Utilities|FlowControl|Delay 0.2)))))
            (:then_1
              (Timeline|Timeline_1 Stop))
            (:then_2
              (Timeline|Timeline_0 Stop))
            (:then_3
              (Variables|Default|SetThrow%20Speed 0.0))
            (:then_4
              (Audio|PlaySound2D "/Game/Audio/SE/Miss_cue.Miss_cue" 1.0 1.0 0.0 0 0))))))))

(event Input|KeyboardEvents|A
  (params (Key :type Key%20Structure :default "None"))
  ;[1 1 1] player movement
  (:Pressed
    (if (Variables|Default|GetPlayer%20Turn%20?)
      (Development|PrintString "press A")
      (if (Variables|Default|GetCanChangeDirection)
        (Variables|Default|SetTurnLeft? true))))
  (:Released
    (if (Variables|Default|GetPlayer%20Turn%20?)
      (Variables|Default|SetTurnLeft? false))))

(event Input|KeyboardEvents|D
  (params (Key :type Key%20Structure :default "None"))
  ;[1 1 1] player movement
  (:Pressed
    (if (Variables|Default|GetPlayer%20Turn%20?)
      (Development|PrintString "press D")
      (if (Variables|Default|GetCanChangeDirection)
        (Variables|Default|SetTurnRight? true))))
  (:Released
    (if (Variables|Default|GetPlayer%20Turn%20?)
      (Variables|Default|SetTurnRight? false))))

(fn ConstructionScript)

(fn Charge)

(fn SwitchTurn
  (if (Utilities|Enum|Equal(Enum) (Variables|Default|GetCurrentTurn) "NewEnumerator0")
    (Variables|Default|SetCurrentTurn "NewEnumerator1")
    (else
      (Variables|Default|SetCurrentTurn "NewEnumerator0"))))