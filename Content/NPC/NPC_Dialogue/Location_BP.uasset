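; Location_BP is a quest location trigger that completes any active quest pointing at it when the player enters its box.
; On overlap it scans the player's ActiveQuests for an ActorReference matching itself and calls QuestComplete on the player.
; It then searches all BP_NPC1 actors and fires EventQuestComplete on those whose QuestRef has the same quest name.
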(event OnComponentBeginOverlap(Box)
  (params (OverlappedComponent :type Primitive%20Component%20Object%20Reference) (OtherActor :type Actor%20Object%20Reference) (OtherComp :type Primitive%20Component%20Object%20Reference) (OtherBodyIndex :type Integer) (bFromSweep :type Boolean) (SweepResult :type Hit%20Result%20Structure%20%28by%20ref%29))
  (bind _asplayer_blue_print (Utilities|Casting|CastToPlayerBluePrint OtherActor))
  (for _array_element (Variables|/Game/Player/PlayerBluePrint.PlayerBluePrint_C|GetActiveQuests _asplayer_blue_print)
    (if (== self (.actorreference (Variables|/Game/NPC/NPC_Dialogue/BP_Quest.BP_Quest_C|GetQuestInfo _array_element)))
      (Default|QuestComplete _asplayer_blue_print _array_element)
      (bind _outactors (Actor|GetAllActorsOfClass "/Game/NPC/NPC_Dialogue/BP_NPC1.BP_NPC1_C"))
      (for _array_element_2 _outactors
        (if (Utilities|Enum|Equal(Enum) (.questname (Variables|/Game/NPC/NPC_Dialogue/BP_Quest.BP_Quest_C|GetQuestInfo _array_element)) (.questname (Variables|/Game/NPC/NPC_Dialogue/BP_NPC1.BP_NPC1_C|GetQuest%20Ref _array_element_2)))
          (Default|EventQuestComplete _array_element_2))))))

(fn ConstructionScript)